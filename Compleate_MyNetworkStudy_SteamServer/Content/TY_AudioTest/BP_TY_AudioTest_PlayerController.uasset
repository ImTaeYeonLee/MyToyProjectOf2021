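; Test player controller for networked voice chat, with the N key wired as push-to-talk to start and stop voice.
; On possess, it waits briefly, then registers its own unique net ID as a remote talker.
; Tick also starts networked voice every frame, working against the key release, and prints whether the local player is talking.
; A local talker registration node is present but unconnected.
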(event EventBeginPlay)

(event EventTick
  (params (DeltaSeconds :type Float%20%28single-precision%29))
  ;[1 1 1] 코멘트
  (Class|AdvancedVoiceLibrary|StartNetworkedVoice)
  (Development|PrintString (Utilities|String|ToString(Boolean) (Class|AdvancedVoiceLibrary|IsLocalPlayerTalking))))

(event EventPossess
  (params (PossessedPawn :type Pawn%20Object%20Reference))
  ;[1 1 1] 코멘트
  (Utilities|FlowControl|Delay 1.0)
  (Class|AdvancedVoiceLibrary|RegisterRemoteTalker (Class|AdvancedSessionsLibrary|GetUniqueNetID self)))

(event Input|KeyboardEvents|V
  (params (Key :type Key%20Structure :default "None")))

(event Input|KeyboardEvents|N
  (params (Key :type Key%20Structure :default "None"))
  (:Pressed
    (Class|AdvancedVoiceLibrary|StartNetworkedVoice))
  (:Released
    (Class|AdvancedVoiceLibrary|StopNetworkedVoice)))

(fn ConstructionScript)