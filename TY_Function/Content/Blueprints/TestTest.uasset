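; Test Blueprint that switches the player between VR and PC modes at runtime.
; BeginPlay applies the VRMod flag, and Tab flips it and reapplies it through ChangeState.
; ChangeState enables or disables the HMD to match, then activates MoveComp, HandComp and GrabComp for VR or PlayerMove and PlayerCameraController for PC, deactivating the other set.
; HMD status printing and a console-command HMD enable remain as unconnected debug nodes.
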(event Custom|ChangeState
  ;[1 1 1] HMD 켜기
  (Class|HeadMountedDisplayFunctionLibrary|EnableHMD (Variables|Default|GetVRMod))
  (if (Variables|Default|GetVRMod)
    (Components|Activation|Activate (Variables|Default|GetmoveComp) false)
    (Components|Activation|Deactivate (Variables|Default|GetplayerMove))
    (else
      (Components|Activation|Deactivate (Variables|Default|GetmoveComp))
      (Components|Activation|Activate (Variables|Default|GetplayerMove) false))))

(event EventBeginPlay
  ;[1 1 1] 콘솔에 명령어를 전달(나 HMD 쓸거야)
  (CallFunction|ChangeState))

(event Collision|EventActorBeginOverlap
  (params (OtherActor :type Actor%20Object%20Reference)))

(event EventTick
  (params (DeltaSeconds :type Float%20%28single-precision%29)))

(event Input|KeyboardEvents|Tab
  (params (Key :type Key%20Structure :default "None"))
  ;[1 1 1] Tab 누르면 HMD 켜고 끄기
  (:Pressed
    (Variables|Default|SetVRMod (not (Variables|Default|GetVRMod)))
    (CallFunction|ChangeState)))

(fn ConstructionScript)